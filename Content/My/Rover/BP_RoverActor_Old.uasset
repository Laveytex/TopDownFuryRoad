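; BP_RoverActor_Old is a drivable rover vehicle that feeds throttle, steering and handbrake input into its vehicle movement component.
; Mouse X and Y rotate the spring arm in yaw and pitch to orbit the camera.
; Pressing W dims the mesh's emissive parameter and releasing it brightens it, creating a new dynamic material instance each time.
; A leftover FlipFlop toggle for that glow never runs.
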(event `InputAxisKey|MouseX`
  (params (AxisValue :type "Float (single-precision)"))
  (`SceneComponent.K2_AddRelativeRotation` (`self.SpringArm`) (`KismetMathLibrary.MakeRotator` 0.0 0.0 AxisValue) false false))

(event `InputAxisKey|MouseY`
  (params (AxisValue :type "Float (single-precision)"))
  (`SceneComponent.K2_AddRelativeRotation` (`self.SpringArm`) (`KismetMathLibrary.MakeRotator` 0.0 AxisValue) false false))

(event `self.ReceiveTick`
  (params (DeltaSeconds :type "Float (single-precision)")))

(event `InputAxis|Throttle`
  (params (AxisValue :type "Float (single-precision)"))
  (`ChaosVehicleMovementComponent.SetThrottleInput` (`self.VehicleMovementComponent`) AxisValue))

(event `Key|W`
  (params (Key :type "Key Structure"))
  (:`Pressed`
    (bind _returnvalue (`PrimitiveComponent.CreateDynamicMaterialInstance` (`self.Mesh`) 0 "/Game/My/Rover/M_Rover_Inst.M_Rover_Inst" "Emiss"))
    (`MaterialInstanceDynamic.SetScalarParameterValue` _returnvalue "Emiss" 1.0))
  (:`Released`
    (bind _returnvalue_2 (`PrimitiveComponent.CreateDynamicMaterialInstance` (`self.Mesh`) 0 "/Game/My/Rover/M_Rover_Inst.M_Rover_Inst" "Emiss"))
    (`MaterialInstanceDynamic.SetScalarParameterValue` _returnvalue_2 "Emiss" 5.0)))

(event `InputAxis|MoveRight`
  (params (AxisValue :type "Float (single-precision)"))
  (`ChaosVehicleMovementComponent.SetSteeringInput` (`self.VehicleMovementComponent`) AxisValue))

(event `InputAction|MoveBrake`
  (params (Key :type "Key Structure"))
  (bind _vehiclemovementcomponent (`self.VehicleMovementComponent`))
  (:`Pressed`
    (`ChaosVehicleMovementComponent.SetHandbrakeInput` _vehiclemovementcomponent true))
  (:`Released`
    (`ChaosVehicleMovementComponent.SetHandbrakeInput` _vehiclemovementcomponent false)))

(fn `UserConstructionScript`)